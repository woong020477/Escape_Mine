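; BP_Boss is a boss actor that alternates between a fire-floor attack and an enemy-spawning pattern.
; A looping timer flips the pattern value, while Tick runs the current pattern behind an execute-once flag that resets after a delay.
; The fire pattern spawns a temporary BP_FireBox, and the other spawns BP_GroundEnemy pairs at fixed points.
; GetDamage lowers HP, and Tick destroys the boss at zero while printing HP for debugging.
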(event `TogglePattern`
  ;[1 1 1] 패턴변경
  (if (== 0 (`self.Patern Value`))
    (set `self.Patern Value` 1)
    (`KismetSystemLibrary.PrintString` "적 생성 패턴")
    (else
      (set `self.Patern Value` 0)
      (`KismetSystemLibrary.PrintString` "불바닥 패턴"))))

(event `self.ReceiveBeginPlay`
  (`KismetSystemLibrary.K2_SetTimer` null "TogglePattern" 11.0 true))

(event `self.ReceiveTick`
  (params (DeltaSeconds :type "Float (single-precision)"))
  (bind _hp (`self.HP`))
  (`|ExecutionSequence`
    (:`then_0`
      (if (not (`self.HasExecuted`))
        (set `self.HasExecuted` true)
        (if (== (`self.Patern Value`) 0)
          (bind _returnvalue (`|SpawnActorFromClass` "/Game/BluePrints/TaskFile/BP_FireBox.BP_FireBox_C" (`KismetMathLibrary.MakeTransform` (-4720.0 -240.0 19.956887) (struct) (19.25 19.25 0.1)) "Undefined" "MultiplyWithRoot" null null))
          (`KismetSystemLibrary.Delay` 7.0)
          (set `self.HasExecuted` false)
          (`self.K2_DestroyActor` _returnvalue)
          (else
            (`|ExecutionSequence`
              (:`then_0`
                (`|SpawnActorFromClass` "/Game/BluePrints/BP_GroundEnemy.BP_GroundEnemy_C" (`KismetMathLibrary.MakeTransform` (-4890.0 -600.0 1040.0)) "Undefined" "MultiplyWithRoot" null null)
                (`KismetSystemLibrary.Delay` 0.2)
                (`|SpawnActorFromClass` "/Game/BluePrints/BP_GroundEnemy.BP_GroundEnemy_C" (`KismetMathLibrary.MakeTransform` (-4890.0 -600.0 1040.0)) "Undefined" "MultiplyWithRoot" null null))
              (:`then_1`
                (`|SpawnActorFromClass` "/Game/BluePrints/BP_GroundEnemy.BP_GroundEnemy_C" (`KismetMathLibrary.MakeTransform` (-4370.0 -600.0 890.0)) "Undefined" "MultiplyWithRoot" null null)
                (`KismetSystemLibrary.Delay` 0.2)
                (`|SpawnActorFromClass` "/Game/BluePrints/BP_GroundEnemy.BP_GroundEnemy_C" (`KismetMathLibrary.MakeTransform` (-4370.0 -600.0 890.0)) "Undefined" "MultiplyWithRoot" null null))
              (:`then_2`
                (`|SpawnActorFromClass` "/Game/BluePrints/BP_GroundEnemy.BP_GroundEnemy_C" (`KismetMathLibrary.MakeTransform` (-4370.0 40.0 890.0)) "Undefined" "MultiplyWithRoot" null null)
                (`KismetSystemLibrary.Delay` 0.2)
                (`|SpawnActorFromClass` "/Game/BluePrints/BP_GroundEnemy.BP_GroundEnemy_C" (`KismetMathLibrary.MakeTransform` (-4370.0 40.0 890.0)) "Undefined" "MultiplyWithRoot" null null))
              (:`then_3`
                (`|SpawnActorFromClass` "/Game/BluePrints/BP_GroundEnemy.BP_GroundEnemy_C" (`KismetMathLibrary.MakeTransform` (-4980.0 40.0 80.0)) "Undefined" "MultiplyWithRoot" null null)
                (`KismetSystemLibrary.Delay` 0.2)
                (`|SpawnActorFromClass` "/Game/BluePrints/BP_GroundEnemy.BP_GroundEnemy_C" (`KismetMathLibrary.MakeTransform` (-4980.0 40.0 80.0)) "Undefined" "MultiplyWithRoot" null null)))
            (`KismetSystemLibrary.Delay` 7.0)
            (set `self.HasExecuted` false)))))
    (:`then_1`
      ;[1 1 1] 액터 HP관련
      (if (<= _hp 0)
        (`self.K2_DestroyActor`)))
    (:`then_2`
      (`KismetSystemLibrary.PrintString` (`KismetStringLibrary.Conv_IntToString` _hp)))))

(fn `GetDamage`
  (params (Damage :type Integer))
  (set `self.HP` (- (`self.HP`) Damage)))

(fn `UserConstructionScript`)