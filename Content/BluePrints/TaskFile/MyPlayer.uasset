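; Player character Blueprint handling health, pickaxe melee combat and death/revive, loading and saving attack damage through BP_GI.
; IA_Attack, gated on pickaxe ownership, alternates two montages as a combo, with notifies advancing the counter and a timer resetting it.
; Capsule overlaps while attacking damage ground enemies, rocks and bosses.
; Hits update the status widget; death pauses the game with a death widget until revive restores HP.
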(event `self.ReceiveTick`
  (params (DeltaSeconds :type "Float (single-precision)"))
  (`self.UpdateHPUI`))

(event `ClickReviveButtonEvent`
  ;[1 1 1] 부활 버튼 클릭
  (`GameplayStatics.SetGamePaused` false)
  (`self.Revive` (stale `OnHitEvent` _returnvalue_2)))

(event `OnHitEvent`
  (params (Damaged :type Integer))
  (bind _returnvalue (`GameplayStatics.GetPlayerController` 0))
  ;[1 1 1] Player 피격
  (`/Game/UI/WBP_PlayerStatusWidget.OnDamageEvent` (`self.UIScreen`))
  (bind _output_get (set `self.HP` (- (`self.HP`) Damaged)))
  (`self.UpdateHPUI`)
  (if (<= _output_get 0)
    ;[1 1 1] HP == 0 일때 사망
    (bind _returnvalue_2 (`|CreateWidget` "/Game/UI/WBP_PlayerDeathWidget.WBP_PlayerDeathWidget_C"))
    (`WidgetBlueprintLibrary.SetInputMode_UIOnlyEx` _returnvalue _returnvalue_2)
    (`UserWidget.AddToViewport` _returnvalue_2 0)
    (set `PlayerController.bShowMouseCursor` true _returnvalue)
    (`GameplayStatics.SetGamePaused` true)))

(event `self.ReceiveBeginPlay`
  ;[1 1 1] 게임 인스턴스 곡괭이 유무, 데미지 현황 불러오기
  (bind _asbp_gi (cast `/Game/BluePrints/BP_GI` (`GameplayStatics.GetGameInstance`)))
  (set `self.AttackDamage` (`/Game/BluePrints/BP_GI.PlayerAttackDamage` _asbp_gi))
  (if (`/Game/BluePrints/BP_GI.PlayerPickaxe?` _asbp_gi)
    (set `self.IsPickaxeVisble` true)
    (`SceneComponent.SetVisibility` (`self.StaticMesh`) true false)
    (else
      (set `self.IsPickaxeVisble` false)))
  ;[1 1 1] 초기 HP 지정
  (set `self.MaxHP` (`self.HP`))
  ;[1 1 1] Player Status 위젯 세팅 및 HP갱신
  (bind _returnvalue (`|CreateWidget` "/Game/UI/WBP_PlayerStatusWidget.WBP_PlayerStatusWidget_C"))
  (bind _output_get (set `self.UIScreen` _returnvalue))
  (`UserWidget.AddToViewport` _output_get 0)
  (`self.UpdateHPUI`))

(event `EnhancedInput|/Game/Input/TaskFolder/IA_Attack`
  (params (ActionValue :type Boolean) (ElapsedSeconds :type "Float (double-precision)") (TriggeredSeconds :type "Float (double-precision)") (InputAction :type "InputAction Object Reference" :default "/Game/Input/TaskFolder/IA_Attack.IA_Attack"))
  (bind _mesh (`self.Mesh`))
  ;[1 1 1] 공격 관련 노드 (몽타주)
  (:`Triggered`
    (if (`self.IsPickaxeVisble`)
      (if (not (`self.IsAttacking`))
        (set `self.IsAttacking` true)
        (switch `int` (`self.comboCnt`)
          (:`0`
            (`|PlayMontage` _mesh "/Game/Animations/Animation_Seq/Montages/Rt_Attack_1.Rt_Attack_1" 1.3
              (:`then`
                (`KismetSystemLibrary.K2_SetTimerDelegate` (delegate `ResetCounter`) 2.5 :!label _label))
              (:`OnNotifyBegin`
                (set `self.comboCnt` (+ (`self.comboCnt`) 1))
                (set `self.IsAttacking` false))))
          (:`1`
            (`|PlayMontage` _mesh "/Game/Animations/Animation_Seq/Montages/Rt_Attack_2.Rt_Attack_2" 1.5
              (:`then`
                (goto _label))
              (:`OnNotifyBegin`
                (set `self.comboCnt` (- (`self.comboCnt`) 1))
                (set `self.IsAttacking` false)))))))))

(event `ResetCounter`
  ;[1 1 1] 공격 관련 노드 (몽타주)
  (set `self.comboCnt` 0)
  (set `self.IsAttacking` false))

(event `self.CapsuleComp.OnComponentBeginOverlap`
  (params (OverlappedComponent :type "PrimitiveComponent Object Reference") (OtherActor :type "Actor Object Reference") (OtherComp :type "PrimitiveComponent Object Reference") (OtherBodyIndex :type Integer) (bFromSweep :type Boolean) (SweepResult :type "HitResult Structure (by ref)"))
  ;[1 1 1] 기본 공격 로직
  (if (`self.IsAttacking`)
    (`|ExecutionSequence`
      (:`then_0`
        (bind _asbp_ground_enemy (cast `/Game/BluePrints/BP_GroundEnemy` OtherActor))
        (`/Game/BluePrints/BP_GroundEnemyFSM.OnDamageProcess` (`/Game/BluePrints/BP_GroundEnemy.BP_GroundEnemyFSM` _asbp_ground_enemy) (`self.GetActorForwardVector`) (`self.AttackDamage`)))
      (:`then_1`
        ;[1 1 1] 바위 HP피해
        (bind _asrock (cast `/Game/BluePrints/TaskFile/Rock` OtherActor))
        (`/Game/BluePrints/TaskFile/Rock.GetDamage` _asrock (`self.AttackDamage`)))
      (:`then_2`
        ;[1 1 1] BossEnemy 공격
        (bind _asbp_boss_enemy (cast `/Game/BluePrints/BP_BossEnemy` OtherActor))
        (`/Game/BluePrints/BP_BossEnemyFSM.OnDamageProcess` (`/Game/BluePrints/BP_BossEnemy.BP_BossEnemyFSM` _asbp_boss_enemy) (`self.GetActorForwardVector`) (`self.AttackDamage`)))
      (:`then_3`
        ;[1 1 1] BossEnemy2 공격
        (bind _asbp_boss_enemy_2 (cast `/Game/BluePrints/BP_BossEnemy2` OtherActor))
        (`/Game/BluePrints/BP_BossEnemy2FSM.OnDamageProcess` (`/Game/BluePrints/BP_BossEnemy2.BP_BossEnemy2FSM` _asbp_boss_enemy_2) (`self.GetActorForwardVector`) (`self.AttackDamage`)))
      (:`then_4`
        ;[1 1 1] 석상 보스 HP피해
        (bind _asbp_boss (cast `/Game/BluePrints/TaskFile/BP_Boss` OtherActor))
        (`/Game/BluePrints/TaskFile/BP_Boss.GetDamage` _asbp_boss (`self.AttackDamage`))))))

(fn `Revive`
  (params (UI :type "Widget Object Reference"))
  (bind _returnvalue (`GameplayStatics.GetPlayerController` 0))
  (set `self.HP` 100)
  (`self.UpdateHPUI`)
  (`Widget.RemoveFromParent` UI)
  (`WidgetBlueprintLibrary.SetInputMode_GameOnly` _returnvalue)
  (`UserWidget.AddToViewport` (`self.UIScreen`) 0)
  (set `PlayerController.bShowMouseCursor` false _returnvalue))

(fn `UpdateDamage`
  (params (Damage :type Integer))
  (bind _output_get (set `self.AttackDamage` Damage))
  (bind _asbp_gi (cast `/Game/BluePrints/BP_GI` (`GameplayStatics.GetGameInstance`)))
  (set `/Game/BluePrints/BP_GI.PlayerAttackDamage` _output_get _asbp_gi))

(fn `UpdateHPUI`
  (`/Game/UI/WBP_PlayerStatusWidget.UpdateHP` (`self.UIScreen`) (`self.HP`) (`self.MaxHP`)))

(fn `UserConstructionScript`)

(fn `UseRecorveryItem`
  (params (RecorverHP :type Integer))
  (if (>= (+ RecorverHP (`self.HP`)) (`self.MaxHP`))
    (set `self.HP` (`self.MaxHP`))
    (else
      (set `self.HP` (+ (`self.HP`) (`local.RecorverHP`)))))
  (`self.UpdateHPUI`))