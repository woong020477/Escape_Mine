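; Destructible rock actor that takes damage and sinks away once its HP is depleted.
; It starts with a fixed HP on BeginPlay, and GetDamage spawns a scaled-down explosion emitter at the rock on each hit before subtracting the damage.
; Tick polls HP and, only when it is strictly below zero, moves the rock down without sweep at DownSpeed, destroying it below a fixed world height.
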(event `self.ReceiveBeginPlay`
  (bind _output_get (set `self.HP` 10)))

(event `self.ReceiveTick`
  (params (DeltaSeconds :type "Float (single-precision)"))
  (bind (_returnvalue_x _returnvalue_y _returnvalue_z) (`KismetMathLibrary.BreakVector` (`self.K2_GetActorLocation`)))
  (if (< (stale `self.ReceiveBeginPlay` _output_get) 0)
    (`self.K2_SetActorLocation` (+ (`self.K2_GetActorLocation`) (* (* (`KismetMathLibrary.Vector_Down`) (`self.DownSpeed`)) (`GameplayStatics.GetWorldDeltaSeconds`))))
    (if (< _returnvalue_z -400.0)
      (`self.K2_DestroyActor`))))

(fn `GetDamage`
  (params (Damage :type Integer))
  (bind _returnvalue (`self.K2_GetActorLocation`))
  (`GameplayStatics.SpawnEmitterAtLocation` "/Game/StarterContent/Particles/P_Explosion.P_Explosion" _returnvalue (`KismetMathLibrary.Conv_VectorToRotator` _returnvalue) (0.5 0.5 0.5))
  (set `self.HP` (- (`self.HP`) Damage)))

(fn `UserConstructionScript`)