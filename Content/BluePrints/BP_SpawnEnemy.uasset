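; BP_SpawnEnemy is a spawn point actor that creates ground or boss enemies on a random timer.
; Its construction script gathers all BP_SpawnEnemy actors, and spawns draw location and rotation from separate random picks among them.
; Tick rerolls the enemy type within the range set by BP_GI's StageStatus.
; Only successful spawn branches restart the timer; the unimplemented Boss1 and invalid types just print, ending the loop.
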(event `self.ReceiveBeginPlay`
  (`self.EnemySpawnTimer` (delegate `CreateEnemy`) :!label _label))

(event `CreateEnemy`
  (bind _output (`|GetArrayItem` (`self.SpawnPoint`) (`KismetMathLibrary.RandomIntegerInRange` 0 (- (`KismetArrayLibrary.Array_Length` (`self.SpawnPoint`)) 1))))
  (bind _returnvalue (`self.K2_GetActorLocation` _output))
  (bind _returnvalue_2 (`self.K2_GetActorRotation` _output))
  ;[1 1 1] 적 타입에 따라 Enemy 스폰
  (switch `int` (`self.EnemyType`)
    (:`Default`
      (`KismetSystemLibrary.PrintString` "적 타입이 지정되지 않았습니다. \n!! BP_SpawnEnemy 참고 !!"))
    (:`0`
      (`|SpawnActorFromClass` "/Game/BluePrints/BP_GroundEnemy.BP_GroundEnemy_C" (`KismetMathLibrary.MakeTransform` _returnvalue _returnvalue_2) "Undefined" "MultiplyWithRoot" null null)
      (goto _label))
    (:`1`
      (`KismetSystemLibrary.PrintString` "보스1번 아직 없음"))
    (:`2`
      (`|SpawnActorFromClass` "/Game/BluePrints/BP_BossEnemy2.BP_BossEnemy2_C" (`KismetMathLibrary.MakeTransform` _returnvalue _returnvalue_2) "Undefined" "MultiplyWithRoot" null null)
      (goto _label))))

(event `self.ReceiveTick`
  (params (DeltaSeconds :type "Float (single-precision)"))
  (bind _asbp_gi (cast `/Game/BluePrints/BP_GI` (`GameplayStatics.GetGameInstance`)))
  (set `self.EnemyType` (`KismetMathLibrary.RandomIntegerInRange` 0 (- (`/Game/BluePrints/BP_GI.StageStatus` _asbp_gi) 1)))
  (`KismetSystemLibrary.Delay` 1.0))

(fn `EnemySpawnTimer`
  (params (Delegate :type Delegate))
  (`KismetSystemLibrary.K2_SetTimerDelegate` Delegate (`KismetMathLibrary.RandomFloatInRange` (`self.Min`) (`self.Max`))))

(fn `UserConstructionScript`
  (bind _outactors (`GameplayStatics.GetAllActorsOfClass` "BP_SpawnEnemy_C"))
  (set `self.SpawnPoint` _outactors))