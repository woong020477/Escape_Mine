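; Actor component that drives the boss enemy through an Idle, Move, Attack, Damage and Die state machine on Tick.
; Move chases the player when a navmesh path exists, otherwise heads to a random reachable point, and switches to Attack in range.
; OnDamageProcess reduces HP, then triggers lerped knockback or death, where the boss sinks and destroys a BP_Wall and itself.
; A shared timer paces state delays, and ABP_BossEnemy plays animations.
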(event `self.ReceiveTick`
  (params (DeltaSeconds :type "Float (single-precision)"))
  (switch `/Game/BluePrints/EBossEnemyState` (`self.EnemyState`)
    (:`NewEnumerator0`
      (`self.IdleState`))
    (:`NewEnumerator1`
      (`self.MoveState`))
    (:`NewEnumerator2`
      (`self.AttackState`))
    (:`NewEnumerator3`
      (`self.DamageState`))
    (:`NewEnumerator4`
      (`self.DieState`))))

(event `self.ReceiveBeginPlay`
  (set `self.HP` 25)
  (bind _returnvalue (`GameplayStatics.GetActorOfClass` "/Game/BluePrints/TaskFile/MyPlayer.MyPlayer_C"))
  (set `self.PlayerTarget` _returnvalue)
  ;[1 1 1] 본인 객체 저장
  (bind _asbp_boss_enemy (cast `/Game/BluePrints/BP_BossEnemy` (`self.GetOwner`)))
  (bind _output_get (set `self.EnemyTarget` _asbp_boss_enemy))
  (bind _asabp_boss_enemy (cast `/Game/Animations/ABP_BossEnemy` (`SkeletalMeshComponent.GetAnimInstance` (`Character.Mesh` _output_get))))
  (set `self.Anim` _asabp_boss_enemy)
  (bind `_asai_컨트롤러` (cast `AIController` (`Pawn.GetController` (`self.EnemyTarget`))))
  (set `self.AI` `_asai_컨트롤러`))

(fn `AttackState`
  ;[1 1 1] 함수 호출 시 Attack Delay Time 시간마다 공격
  (bind _isfinish_ (`self.FlowTime` (`self.AttackDelayTime`)))
  (if _isfinish_
    (`/Game/Animations/ABP_BossEnemy.PlayAttackAnim` (`self.Anim`))
    ;[1 1 1] Attack Range 벗어났을 때 Move State로 전환
    (if (> (`KismetMathLibrary.Vector_Distance` (`Actor.K2_GetActorLocation` (`self.PlayerTarget`)) (`Actor.K2_GetActorLocation` (`self.EnemyTarget`))) (`self.AttackRange`))
      (set `self.EnemyState` "NewEnumerator1"))))

(fn `CorrectRotation`
  (params (InterpSpeed :type "Float (double-precision)"))
  (bind _enemytarget (`self.EnemyTarget`))
  (bind (_returnvalue_roll _returnvalue_pitch _returnvalue_yaw) (`KismetMathLibrary.BreakRotator` (`Pawn.GetControlRotation` _enemytarget)))
  (bind (_returnvalue_roll_2 _returnvalue_pitch_2 _returnvalue_yaw_2) (`KismetMathLibrary.BreakRotator` (`Pawn.GetControlRotation` _enemytarget)))
  (`Actor.K2_SetActorRotation` (`self.EnemyTarget`) (`KismetMathLibrary.MakeRotator` 0.0 0.0 (`KismetMathLibrary.FInterpTo` _returnvalue_yaw _returnvalue_yaw_2 (`GameplayStatics.GetWorldDeltaSeconds`) (`local.InterpSpeed`))) false))

(fn `DamageState`
  (if (`self.KnockBackPlaying`)
    (`self.Knock Back`))
  ;[1 1 1] 일정 시간 후 Idle State 전환
  (bind _isfinish_ (`self.FlowTime` (`self.DamageDelayTime`)))
  (if _isfinish_
    (set `self.EnemyState` "NewEnumerator0")))

(fn `DieState`
  (bind (_returnvalue_x _returnvalue_y _returnvalue_z) (`KismetMathLibrary.BreakVector` (`Actor.K2_GetActorLocation` (`self.EnemyTarget`))))
  ;[1 1 1] 죽어서 아래로 내려감
  (`Actor.K2_SetActorLocation` (`self.EnemyTarget`) (+ (`Actor.K2_GetActorLocation` (`self.EnemyTarget`)) (* (* (`KismetMathLibrary.Vector_Down`) (`self.Die Speed`)) (`GameplayStatics.GetWorldDeltaSeconds`))) false false)
  (if (< _returnvalue_z -200.0)
    (bind _outactors (`GameplayStatics.GetAllActorsOfClass` "/Game/BluePrints/BP_Wall.BP_Wall_C"))
    (if (> (`KismetArrayLibrary.Array_Length` _outactors) 0)
      (`Actor.K2_DestroyActor` (`|GetArrayItem` _outactors)))
    (`Actor.K2_DestroyActor` (`self.EnemyTarget`))))

(fn `FindAndMove`
  (locals (Start :type "Vector Structure") (End :type "Vector Structure"))
  (set `local.Start` (`Actor.K2_GetActorLocation` (`self.EnemyTarget`)))
  (set `local.End` (`Actor.K2_GetActorLocation` (`self.PlayerTarget`)))
  ;[1 1 1] 미리 길을 지정해둔다
  (bind _returnvalue (`NavigationSystemV1.FindPathToLocationSynchronously` (`local.Start`) (`local.End`) null null))
  ;[1 1 1] 목적지에 갈 수 있는가?
  (if (> (`NavigationPath.GetPathLength` _returnvalue) 0.0)
    ;[1 1 1] Player 위치로 이동
    (`AIController.MoveToLocation` (`self.AI`) (`local.End`) -1.0 true true false true null true)
    (else
      ;[1 1 1] 랜덤 위치로 이동
      (bind _returnvalue_2 (`AIController.MoveToLocation` (`self.AI`) (`self.RandomDestination`) -1.0 true true false true null true))
      (switch `EPathFollowingRequestResult` _returnvalue_2
        (:`Failed`
          _)
        (:`AlreadyAtGoal`
          _))
      (`self.FindPath`))))

(fn `FindPath`
  (set `self.RandomDestination` (`NavigationSystemV1.K2_GetRandomReachablePointInRadius` (`Actor.K2_GetActorLocation` (`self.EnemyTarget`)) 1000.0 null null)))

(fn `FlowTime`
  (params (DelayTime :type "Float (double-precision)"))
  (returns (`IsFinish?` :type Boolean))
  (bind _output_get (set `self.CurrentTime` (+ (`self.CurrentTime`) (`GameplayStatics.GetWorldDeltaSeconds`))))
  (if (> _output_get (`local.DelayTime`))
    (set `self.CurrentTime` 0.0)
    (return true)
    (else
      (return false))))

(fn `GetRandomPositionNavMesh`
  (params (CenterLocation :type "Vector Structure") (Radius :type "Float (double-precision)"))
  (returns (`FindPath?` :type Boolean) (Destination :type "Vector Structure"))
  (bind (_randomlocation _returnvalue) (`NavigationSystemV1.K2_GetRandomReachablePointInRadius` CenterLocation Radius null null))
  (return _returnvalue _randomlocation))

(fn `IdleState`
  (bind _isfinish_ (`self.FlowTime` (`self.IdleDelayTime`)))
  (if _isfinish_
    (set `self.EnemyState` "NewEnumerator1")
    (`self.FindPath`)))

(fn `Knock Back`
  ;[1 1 1] 넉백
  (`Actor.K2_SetActorLocation` (`self.EnemyTarget`) (`self.Lerp`) true false)
  (if (< (`KismetMathLibrary.Vector_Distance` (`Actor.K2_GetActorLocation` (`self.EnemyTarget`)) (`self.EndPoint`)) (`self.KnockBackStopRange`))
    (`Actor.K2_SetActorLocation` (`self.EnemyTarget`) (`self.EndPoint`) false false)
    (set `self.KnockBackPlaying` false)))

(fn `Lerp`
  (returns (Location :type "Vector Structure"))
  (return (`KismetMathLibrary.VLerp` (`Actor.K2_GetActorLocation` (`self.EnemyTarget`)) (`self.EndPoint`) (* (`self.KnockBackPower`) (`GameplayStatics.GetWorldDeltaSeconds`)))))

(fn `MoveState`
  (locals (Distance :type "Float (double-precision)") (Direction :type "Vector Structure"))
  (bind _returnvalue (- (`Actor.K2_GetActorLocation` (`self.PlayerTarget`)) (`Actor.K2_GetActorLocation` (`self.EnemyTarget`))))
  (`self.CorrectRotation` 10.0)
  (set `local.Distance` (`KismetMathLibrary.VSize` _returnvalue))
  (set `local.Direction` (`KismetMathLibrary.Normal` _returnvalue))
  (`self.FindAndMove`)
  (if (< (`local.Distance`) (`self.AttackRange`))
    (set `self.EnemyState` "NewEnumerator2")
    (set `self.CurrentTime` (`self.AttackDelayTime`))
    (`Controller.StopMovement` (`self.AI`))))

(fn `OnDamageProcess`
  (params (HitDirection :type "Vector Structure") (AttackDamage :type Integer))
  (set `self.Hit Direction` HitDirection)
  (`Controller.StopMovement` (`self.AI`))
  (set `self.CurrentTime` 0.0)
  (bind _output_get (set `self.HP` (- (`self.HP`) AttackDamage)))
  (if (> _output_get 0)
    (set `self.EnemyState` "NewEnumerator3")
    (set `self.KnockBackPlaying` true)
    (bind _output_get_2 (set `self.StartPoint` (`Actor.K2_GetActorLocation` (`self.EnemyTarget`))))
    (set `self.EndPoint` (+ _output_get_2 (* (`self.Hit Direction`) (`self.KnockBackDistance`))))
    (`/Game/Animations/ABP_BossEnemy.PlayDamageAnim` (`self.Anim`))
    (else
      (set `self.EnemyState` "NewEnumerator4")
      (`PrimitiveComponent.SetCollisionEnabled` (`Character.CapsuleComponent` (`self.EnemyTarget`)) "NoCollision")
      (`/Game/Animations/ABP_BossEnemy.PlayDieAnim` (`self.Anim`)))))

(fn `P0vt`
  (returns (ReturnValue :type "Vector Structure"))
  (return (+ (* (* (`self.Hit Direction`) (`self.KnockBackPower`)) (`GameplayStatics.GetWorldDeltaSeconds`)) (`Actor.K2_GetActorLocation` (`self.EnemyTarget`)))))