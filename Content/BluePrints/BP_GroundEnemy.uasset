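; BP_GroundEnemy is an enemy actor that chases the player and explodes when its HP runs out.
; BeginPlay sets HP to 1 and caches the MyPlayer actor as its target.
; Each Tick moves it straight toward the target at Speed with an unswept SetActorLocation, without navigation.
; It spawns P_Explosion and destroys itself at zero HP, or is destroyed silently if the target is invalid.
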(event `self.ReceiveTick`
  (params (DeltaSeconds :type "Float (single-precision)"))
  (`/Engine/EditorBlueprintResources/StandardMacros.IsValid` (`self.PlayerTarget`) ; Player가 없으면 바로 삭제
    (:`Is Valid`
      ;[1 1 1] HP가 0보다 작거나 같을경우 폭발이펙트 출력 후 제거, 0보다 클 경우 추적
      (if (<= (`self.HP`) 0)
        (`GameplayStatics.SpawnEmitterAtLocation` "/Game/StarterContent/Particles/P_Explosion.P_Explosion")
        (`self.K2_DestroyActor`)
        (else
          ;[1 1 1] Vector 계산
          (set `self.Direction` (`KismetMathLibrary.Normal` (- (`self.K2_GetActorLocation` (`self.PlayerTarget`)) (`self.K2_GetActorLocation`))))
          (`self.K2_SetActorLocation` (+ (* DeltaSeconds (* (`self.Direction`) (`self.Speed`))) (`self.K2_GetActorLocation`))) ; 추적
        )))
    (:`Is Not Valid`
      (`self.K2_DestroyActor`))))

(event `self.ReceiveBeginPlay`
  ;[1 1 1] 기본값 세팅
  (set `self.HP` 1)
  (bind _returnvalue (`GameplayStatics.GetActorOfClass` "/Game/BluePrints/TaskFile/MyPlayer.MyPlayer_C"))
  (set `self.PlayerTarget` _returnvalue))

(fn `UserConstructionScript`)