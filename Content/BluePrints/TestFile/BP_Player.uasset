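; BP_Player is a player character Blueprint that handles look, movement, jump, crouch and sprint through Enhanced Input.
; BeginPlay adds the IMP_Player mapping context to the local player's input subsystem.
; Movement follows the control rotation, while look input drives controller yaw and pitch.
; Jump and crouch use built-in Character functions, and sprint switches max walk speed and sets an IsSprinting flag.
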(event `self.ReceiveBeginPlay`
  (bind _asplayer_controller (cast `PlayerController` (`self.GetController`)))
  (bind _returnvalue (pcsubsystem `EnhancedInputLocalPlayerSubsystem` _asplayer_controller))
  (`/Engine/EditorBlueprintResources/StandardMacros.IsValid` _returnvalue
    (:`Is Valid`
      (`EnhancedInputSubsystemInterface.AddMappingContext` _returnvalue "/Game/Input/TestBluePrintFolder/IMP_Player.IMP_Player" 0 (struct)))))

(event `EnhancedInput|/Game/Input/TestBluePrintFolder/IA_Lookaround`
  (params (ActionValue :type "Vector2D Structure") (ElapsedSeconds :type "Float (double-precision)") (TriggeredSeconds :type "Float (double-precision)") (InputAction :type "InputAction Object Reference" :default "/Game/Input/TestBluePrintFolder/IA_Lookaround.IA_Lookaround"))
  ;[1 1 1] 주변을 돌아보는 입력
  (:`Triggered`
    (`self.AddControllerYawInput` ActionValue_X)
    (`self.AddControllerPitchInput` ActionValue_Y)))

(event `EnhancedInput|/Game/Input/TestBluePrintFolder/IA_movement`
  (params (ActionValue :type "Vector2D Structure") (ElapsedSeconds :type "Float (double-precision)") (TriggeredSeconds :type "Float (double-precision)") (InputAction :type "InputAction Object Reference" :default "/Game/Input/TestBluePrintFolder/IA_movement.IA_movement"))
  (bind (_returnvalue_roll _returnvalue_pitch _returnvalue_yaw) (`KismetMathLibrary.BreakRotator` (`self.GetControlRotation`)))
  (bind (_returnvalue_roll_2 _returnvalue_pitch_2 _returnvalue_yaw_2) (`KismetMathLibrary.BreakRotator` (`self.GetControlRotation`)))
  ;[1 1 1] 움직임 입력
  (:`Triggered`
    (`self.AddMovementInput` (`KismetMathLibrary.GetRightVector` (`KismetMathLibrary.MakeRotator` _returnvalue_roll_2 0.0 _returnvalue_yaw_2)) ActionValue_X)
    (`self.AddMovementInput` (`KismetMathLibrary.GetForwardVector` (`KismetMathLibrary.MakeRotator` 0.0 0.0 _returnvalue_yaw)) ActionValue_Y)))

(event `EnhancedInput|/Game/Input/TestBluePrintFolder/IA_Jump`
  (params (ActionValue :type Boolean) (ElapsedSeconds :type "Float (double-precision)") (TriggeredSeconds :type "Float (double-precision)") (InputAction :type "InputAction Object Reference" :default "/Game/Input/TestBluePrintFolder/IA_Jump.IA_Jump"))
  ;[1 1 1] 점프
  (:`Started`
    (`self.Jump`))
  (:`Completed`
    (`self.StopJumping`)))

(event `EnhancedInput|/Game/Input/TestBluePrintFolder/IA_Crouch`
  (params (ActionValue :type Boolean) (ElapsedSeconds :type "Float (double-precision)") (TriggeredSeconds :type "Float (double-precision)") (InputAction :type "InputAction Object Reference" :default "/Game/Input/TestBluePrintFolder/IA_Crouch.IA_Crouch"))
  ;[1 1 1] 기어다니기
  (:`Triggered`
    (`self.Crouch`))
  (:`Completed`
    (`self.UnCrouch`)))

(event `EnhancedInput|/Game/Input/TestBluePrintFolder/IA_Sprint`
  (params (ActionValue :type Boolean) (ElapsedSeconds :type "Float (double-precision)") (TriggeredSeconds :type "Float (double-precision)") (InputAction :type "InputAction Object Reference" :default "/Game/Input/TestBluePrintFolder/IA_Sprint.IA_Sprint"))
  (bind _charactermovement (`self.CharacterMovement`))
  ;[1 1 1] 달리기
  (:`Triggered`
    (set `CharacterMovementComponent.MaxWalkSpeed` 600.0 _charactermovement) ; 달리기
    (set `self.Is Sprinting` true))
  (:`Completed`
    (set `CharacterMovementComponent.MaxWalkSpeed` 450.0 _charactermovement) ; 걷기
    (set `self.Is Sprinting` false)))

(fn `UserConstructionScript`)