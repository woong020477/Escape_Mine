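; BP_BossSpawn is a one-shot spawner that creates the boss for the current stage.
; One second after BeginPlay it switches on StageStatus from BP_GI.
; Only stage 3 spawns BP_BossEnemy2, at triple scale; stages 1 and 2 print placeholders and fire an event dispatcher, before the spawner destroys itself.
; The construction script sets SpawnPoint to the first BP_BossSpawn found, not explicitly to self.
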(event `self.ReceiveBeginPlay`
  (bind _spawnpoint (`self.SpawnPoint`))
  (bind _asbp_gi (cast `/Game/BluePrints/BP_GI` (`GameplayStatics.GetGameInstance`)))
  (`KismetSystemLibrary.Delay` 1.0)
  ;[1 1 1] 스테이지 상태에 따라 Boss 스폰
  (switch `int` (`/Game/BluePrints/BP_GI.StageStatus` _asbp_gi)
    (:`Default`
      (`KismetSystemLibrary.PrintString` "적 타입이 지정되지 않았습니다. \n!! BP_SpawnEnemy 참고 !!"))
    (:`1`
      (`KismetSystemLibrary.PrintString` "보스0번 없음")
      (`self.EventDispatcher` :!label _label))
    (:`2`
      (`KismetSystemLibrary.PrintString` "보스1번 아직 없음")
      (goto _label))
    (:`3`
      (`|SpawnActorFromClass` "/Game/BluePrints/BP_BossEnemy2.BP_BossEnemy2_C" (`KismetMathLibrary.MakeTransform` (`self.K2_GetActorLocation` _spawnpoint) (`self.K2_GetActorRotation` _spawnpoint) (3.0 3.0 3.0)) "Undefined" "MultiplyWithRoot" null null)))
  (`self.K2_DestroyActor`))

(fn `UserConstructionScript`
  (bind _returnvalue (`GameplayStatics.GetActorOfClass` "BP_BossSpawn_C"))
  (set `self.SpawnPoint` _returnvalue))