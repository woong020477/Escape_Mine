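; BP_ToBossPortal is a portal actor that sends the player to a Temple level.
; It finds the player on BeginPlay and reacts only when that actor overlaps its Box.
; The overlap updates the stage status on BP_GI, then opens TempleLevel while the status is below the final threshold.
; Otherwise, it sets the status back one step below that threshold and opens TempleFinalLevel.
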(event `self.ReceiveBeginPlay`
  (bind _returnvalue (`GameplayStatics.GetActorOfClass` "/Game/BluePrints/TaskFile/MyPlayer.MyPlayer_C"))
  (set `self.MyPlayer` _returnvalue))

(event `self.Box.OnComponentBeginOverlap`
  (params (OverlappedComponent :type "PrimitiveComponent Object Reference") (OtherActor :type "Actor Object Reference") (OtherComp :type "PrimitiveComponent Object Reference") (OtherBodyIndex :type Integer) (bFromSweep :type Boolean) (SweepResult :type "HitResult Structure (by ref)"))
  (if (== OtherActor (`self.MyPlayer`))
    (`self.MoveToNextMap`)))

(event `MoveToNextMap`
  (bind _asbp_gi (cast `/Game/BluePrints/BP_GI` (`GameplayStatics.GetGameInstance`)))
  (`/Game/BluePrints/BP_GI.UpdateStageStatus` _asbp_gi)
  (if (< (`/Game/BluePrints/BP_GI.StageStatus` _asbp_gi) 4)
    (`GameplayStatics.OpenLevelBySoftObjectPtr` "/Game/Levels/TempleLevel.TempleLevel")
    (else
      (set `/Game/BluePrints/BP_GI.StageStatus` 3 _asbp_gi)
      (`GameplayStatics.OpenLevelBySoftObjectPtr` "/Game/Levels/TempleFinalLevel.TempleFinalLevel"))))

(fn `UserConstructionScript`)